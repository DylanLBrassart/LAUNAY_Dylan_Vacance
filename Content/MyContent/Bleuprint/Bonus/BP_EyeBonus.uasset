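; BP_EyeBonus is a pickup actor that grants the player the Eye bonus.
; Its TriggerZone overlap events show and hide a PressEToGet prompt for BP_Player.
; The Eye event, not called within this graph, sets the player's EyeCollected flag and reveals their Eye component.
; It then displays the UI_Eye widget under UI-only input for a short delay, restores game input and destroys itself.
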(event OnComponentBeginOverlap(TriggerZone)
  (params (OverlappedComponent :type Primitive%20Component%20Object%20Reference) (OtherActor :type Actor%20Object%20Reference) (OtherComp :type Primitive%20Component%20Object%20Reference) (OtherBodyIndex :type Integer) (bFromSweep :type Boolean) (SweepResult :type Hit%20Result%20Structure%20%28by%20ref%29))
  ;[1 1 1] Show Interact
  (Utilities|Casting|CastToBP_Player OtherActor)
  (Development|SetHiddeninGame (Variables|Default|GetPress%20E%20To%20Get) false false))

(event OnComponentEndOverlap(TriggerZone)
  (params (OverlappedComponent :type Primitive%20Component%20Object%20Reference) (OtherActor :type Actor%20Object%20Reference) (OtherComp :type Primitive%20Component%20Object%20Reference) (OtherBodyIndex :type Integer))
  ;[1 1 1] Show Interact
  (Utilities|Casting|CastToBP_Player OtherActor)
  (Development|SetHiddeninGame (Variables|Default|GetPress%20E%20To%20Get) true false))

(event Custom|Eye
  ;[1 1 1] modifie les pv et supprime l'acteur
  (bind _asbp_player (Utilities|Casting|CastToBP_Player (Game|GetPlayerCharacter 0)))
  (Variables|/Game/MyContent/Bleuprint/BP_Player.BP_Player_C|SetEyeCollected? _asbp_player true)
  (Rendering|SetVisibility (Variables|/Game/MyContent/Bleuprint/BP_Player.BP_Player_C|GetEye _asbp_player) true false)
  (bind _returnvalue (UserInterface|CreateWidget "/Game/MyContent/UI/UI_Eye.UI_Eye_C"))
  (UserInterface|Viewport|AddtoViewport _returnvalue 0)
  (Input|SetInputModeUIOnly (Game|GetPlayerController 0) 0 "DoNotLock" false)
  (Utilities|FlowControl|Delay 2.0)
  (Input|SetInputModeGameOnly (Game|GetPlayerController 0) false)
  (Widget|RemovefromParent _returnvalue)
  (Actor|DestroyActor))

(fn ConstructionScript)