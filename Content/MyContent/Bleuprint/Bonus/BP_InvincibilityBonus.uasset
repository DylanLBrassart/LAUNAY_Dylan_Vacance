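; BP_InvincibilityBonus is a pickup actor that grants invincibility to the player.
; Its TriggerZone shows the PressEToGet prompt while a BP_Player overlaps it and hides it when the overlap ends.
; The Invinsibility event, which is not called within this Blueprint, sets the Invincibility flag on player character 0 and destroys the pickup.
; The Blueprint has no timer or reset for the flag.
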(event OnComponentBeginOverlap(TriggerZone)
  (params (OverlappedComponent :type Primitive%20Component%20Object%20Reference) (OtherActor :type Actor%20Object%20Reference) (OtherComp :type Primitive%20Component%20Object%20Reference) (OtherBodyIndex :type Integer) (bFromSweep :type Boolean) (SweepResult :type Hit%20Result%20Structure%20%28by%20ref%29))
  ;[1 1 1] Show Interact
  (Utilities|Casting|CastToBP_Player OtherActor)
  (Development|SetHiddeninGame (Variables|Default|GetPress%20E%20To%20Get) false false))

(event OnComponentEndOverlap(TriggerZone)
  (params (OverlappedComponent :type Primitive%20Component%20Object%20Reference) (OtherActor :type Actor%20Object%20Reference) (OtherComp :type Primitive%20Component%20Object%20Reference) (OtherBodyIndex :type Integer))
  ;[1 1 1] Show Interact
  (Utilities|Casting|CastToBP_Player OtherActor)
  (Development|SetHiddeninGame (Variables|Default|GetPress%20E%20To%20Get) true false))

(event Custom|Invinsibility
  ;[1 1 1] modifie la variable invincible?
  (bind _asbp_player (Utilities|Casting|CastToBP_Player (Game|GetPlayerCharacter 0)))
  (Variables|/Game/MyContent/Bleuprint/BP_Player.BP_Player_C|SetInvincibility? _asbp_player true)
  (Actor|DestroyActor))

(fn ConstructionScript)