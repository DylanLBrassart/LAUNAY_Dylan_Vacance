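; Game mode that sets up the HUD and handles the player's game over.
; BeginPlay adds the UI_Hud widget to the viewport.
; Tick polls BP_Player's Hp and, once when it equals zero, enables mesh physics simulation, shows the cursor and switches to UI-only input.
; Short delays then stagger showing the UI_GameOver widget and pausing the game.
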(event EventBeginPlay
  ;[1 1 1] UI Hud
  (bind _returnvalue (UserInterface|CreateWidget "/Game/MyContent/UI/Hud/UI_Hud.UI_Hud_C"))
  (UserInterface|Viewport|AddtoViewport _returnvalue 0))

(event EventTick
  (params (DeltaSeconds :type Float%20%28single-precision%29))
  (bind _returnvalue (Game|GetPlayerController 0))
  ;[1 1 1] lance le gameover si les hp du joueur = 0 lance une animation mets les input et le cursor en ui vrée le widget et met le jeu en pause
  (bind _asbp_player (Utilities|Casting|CastToBP_Player (Game|GetPlayerCharacter 0)))
  (if (== (Variables|/Game/MyContent/Bleuprint/BP_Player.BP_Player_C|GetHp _asbp_player) 0)
    (Utilities|FlowControl|DoOnce false
      (:Completed
        (Physics|SetSimulatePhysics (Variables|/Script/Engine.Character|GetMesh _asbp_player) true)
        (Variables|/Script/Engine.PlayerController|SetbShowMouseCursor _returnvalue true)
        (Input|SetInputModeUIOnly _returnvalue 0 "DoNotLock" false)
        (Utilities|FlowControl|Delay 0.2)
        (bind _returnvalue_2 (UserInterface|CreateWidget "/Game/MyContent/UI/UI_GameOver.UI_GameOver_C"))
        (UserInterface|Viewport|AddtoViewport _returnvalue_2 0)
        (Utilities|FlowControl|Delay 0.5)
        (Game|SetGamePaused true)))))

(fn ConstructionScript)