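; Cutscene platform that carries its cube mesh along a spline once the player who has collected the eye touches it.
; A box overlap casts to BP_Player, checks EyeCollected, then plays a timeline whose Time output, scaled by spline length, sets the cube's world location.
; Rotation always samples the spline's start in local space with pitch zeroed, so the cube does not turn along the path.
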(event OnComponentBeginOverlap(Box)
  (params (OverlappedComponent :type Primitive%20Component%20Object%20Reference) (OtherActor :type Actor%20Object%20Reference) (OtherComp :type Primitive%20Component%20Object%20Reference) (OtherBodyIndex :type Integer) (bFromSweep :type Boolean) (SweepResult :type Hit%20Result%20Structure%20%28by%20ref%29))
  (bind _spline (Variables|Default|GetSpline))
  (bind _spline_2 (Variables|Default|GetSpline))
  (bind _cube1 (Variables|Default|GetCube1))
  (bind _returnvalue (Spline|GetRotationatDistanceAlongSpline _spline 0.0 "Local"))
  (bind _returnvalue_2 (Spline|GetRotationatDistanceAlongSpline _spline_2 0.0 "Local"))
  ;[1 1 1] verifie si on est en contact avec la plateforme et si on a recuperer l'eye
  (bind _asbp_player (Utilities|Casting|CastToBP_Player OtherActor))
  (if (Variables|/Game/MyContent/Bleuprint/BP_Player.BP_Player_C|GetEyeCollected? _asbp_player)
    ;[1 1 1] déplace la plateforme en fonction du spline
    (Transformation|SetRelativeRotation (Variables|Default|GetCube1) (Math|Rotator|MakeRotator (.roll _returnvalue) 0.0 (.yaw _returnvalue)) false false)
    (bind _time (Timeline|Timeline Play)
      (:Update
        (Transformation|SetWorldLocation _cube1 (Spline|GetLocationatDistanceAlongSpline _spline_2 (* _time (Spline|GetSplineLength _spline_2)) "World") false false)
        (Transformation|SetWorldRotation _cube1 (Math|Rotator|MakeRotator (.roll _returnvalue_2) 0.0 (.yaw _returnvalue_2)) false false)))))

(fn ConstructionScript)