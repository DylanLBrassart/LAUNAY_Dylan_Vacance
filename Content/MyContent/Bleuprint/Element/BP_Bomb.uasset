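; Timed bomb actor that explodes a few seconds after spawning, damages enemies and then destroys itself.
; BeginPlay runs a delay chain that briefly scales up the collision sphere as the blast area, alongside a 2D sound and particle effect.
; Any BP_MasterEnemy that begins overlapping the sphere, even before detonation, loses a fixed amount of HpEnnemie through direct subtraction.
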(event OnComponentBeginOverlap(SphereCollision)
  (params (OverlappedComponent :type Primitive%20Component%20Object%20Reference) (OtherActor :type Actor%20Object%20Reference) (OtherComp :type Primitive%20Component%20Object%20Reference) (OtherBodyIndex :type Integer) (bFromSweep :type Boolean) (SweepResult :type Hit%20Result%20Structure%20%28by%20ref%29))
  ;[1 1 1] degat
  (bind _asbp_master_enemy (Utilities|Casting|CastToBP_MasterEnemy OtherActor))
  (Variables|/Game/MyContent/Ai/BP_MasterEnemy.BP_MasterEnemy_C|SetHpEnnemie _asbp_master_enemy (- (Variables|/Game/MyContent/Ai/BP_MasterEnemy.BP_MasterEnemy_C|GetHpEnnemie _asbp_master_enemy) 1e+02)))

(event EventBeginPlay
  (bind _spherecollision (Variables|Default|GetSphereCollision))
  ;[1 1 1] explosion
  (Utilities|FlowControl|Delay 3.0)
  (Transformation|SetWorldScale3D _spherecollision "20.000000,20.000000,20.000000")
  (Audio|PlaySound2D "/Game/MyContent/Audio/SFX/ExplosionSFX.ExplosionSFX" 1.0 1.0 0.0 0 0)
  (Components|Activation|Activate (Variables|Default|GetParticleSystem) false)
  (Utilities|FlowControl|Delay 0.3)
  (Transformation|SetWorldScale3D _spherecollision "1.000000,1.000000,1.000000")
  (Utilities|FlowControl|Delay 0.2)
  (Actor|DestroyActor))

(fn ConstructionScript)