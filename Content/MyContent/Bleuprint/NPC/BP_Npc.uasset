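; NPC actor that shows a "press E to chat" prompt while the player is inside its trigger zone and runs a linear dialogue.
; Each Talk call steps through the Dialogue array and writes the line into a UI_Dialogue widget, created and added to the viewport only when none is valid.
; Past the last line, it removes the widget, resets the index and sets the player's walk and sprint speeds.
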(event OnComponentBeginOverlap(TriggerZone)
  (params (OverlappedComponent :type Primitive%20Component%20Object%20Reference) (OtherActor :type Actor%20Object%20Reference) (OtherComp :type Primitive%20Component%20Object%20Reference) (OtherBodyIndex :type Integer) (bFromSweep :type Boolean) (SweepResult :type Hit%20Result%20Structure%20%28by%20ref%29))
  ;[1 1 1] Show Interact
  (Utilities|Casting|CastToBP_Player OtherActor)
  (Development|SetHiddeninGame (Variables|Default|GetPress%20E%20To%20chat) false false))

(event OnComponentEndOverlap(TriggerZone)
  (params (OverlappedComponent :type Primitive%20Component%20Object%20Reference) (OtherActor :type Actor%20Object%20Reference) (OtherComp :type Primitive%20Component%20Object%20Reference) (OtherBodyIndex :type Integer))
  ;[1 1 1] Show Interact
  (Utilities|Casting|CastToBP_Player OtherActor)
  (Development|SetHiddeninGame (Variables|Default|GetPress%20E%20To%20chat) true false))

(event EventTalk
  ;[1 1 1] utilise un tableau de reponse, affiche et retire le widget
  (Math|Integer|IncrementInt (Variables|Default|Gettalkindex)
    (:%20%20
      (if (< (Variables|Default|Gettalkindex) (Utilities|Array|Length (Variables|Default|Getdialogue)))
        (Variables|Default|GetUI
          (:then
            _)
          (:else
            (bind _returnvalue (UserInterface|CreateWidget "/Game/MyContent/Bleuprint/NPC/UI_Dialogue.UI_Dialogue_C" (Game|GetPlayerController 0)))
            (bind _output_get (Variables|Default|SetUI _returnvalue))
            (UserInterface|Viewport|AddtoViewport _output_get 0)))
        (Rendering|Components|TextRender|SetText (Variables|/Game/MyContent/Bleuprint/NPC/UI_Dialogue.UI_Dialogue_C|GetTalkText (Variables|Default|GetUI)) (Utilities|Text|ToText(String) (Utilities|Array|Get(acopy) (Variables|Default|Getdialogue) (Variables|Default|Gettalkindex))))
        (else
          (Widget|RemovefromParent (Variables|Default|GetUI))
          (Variables|Default|Settalkindex -1)
          (bind _asbp_player (Utilities|Casting|CastToBP_Player (Game|GetPlayerCharacter 0)))
          (Variables|/Game/MyContent/Bleuprint/BP_Player.BP_Player_C|SetSprintSpeed _asbp_player 1.2e+03)
          (Variables|/Game/MyContent/Bleuprint/BP_Player.BP_Player_C|SetWalkSpeed _asbp_player 6e+02))))))

(fn ConstructionScript)