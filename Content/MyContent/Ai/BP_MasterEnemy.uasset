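; BP_MasterEnemy is an enemy Blueprint, named as a master class, that provides health state and a floating health bar.
; BeginPlay fills current HP to its maximum and sets the character's walk speed.
; Every Tick casts the widget component's content to UI_HpEnemy and writes the HP ratio to its progress bar.
; The same Tick billboards the widget toward the player camera with a look-at rotation, keeping it readable from any position.
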(event EventBeginPlay
  (Variables|Default|SetHpEnnemie (Variables|Default|GetHpMaxEnnemie))
  (Variables|/Script/Engine.CharacterMovementComponent|SetMaxWalkSpeed (Variables|Character|GetCharacterMovement) 5.5e+02))

(event EventTick
  (params (DeltaSeconds :type Float%20%28single-precision%29))
  (bind _widget_hpennemie (Variables|Default|GetWidget%20HpEnnemie))
  ;[1 1 1] widget flotant et reste visible pour le joueur peu importe sa position
  (bind _asui_hp_enemy (Utilities|Casting|CastToUI_HpEnemy (UserInterface|GetWidget (Variables|Default|GetWidget%20HpEnnemie))))
  (Progress|SetPercent (Variables|/Game/MyContent/UI/UI_HpEnemy.UI_HpEnemy_C|GetProgressBar_HpEnnemie _asui_hp_enemy) (/ (Variables|Default|GetHpEnnemie) (Variables|Default|GetHpMaxEnnemie)))
  (Transformation|SetWorldRotation _widget_hpennemie (Math|Rotator|FindLookatRotation (Transformation|GetWorldLocation _widget_hpennemie) (Transformation|GetWorldLocation (Variables|/Script/Engine.PlayerCameraManager|GetTransformComponent (Game|GetPlayerCameraManager 0)))) false false))

(fn ConstructionScript)